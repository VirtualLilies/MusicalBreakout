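; NeonBar is an Arkanoid level piece that animates into place and flickers in height.
; Construction randomizes its InterpToMovement duration; the game mode's start-game event restarts that movement.
; A looping timer with a random interval randomizes the cube's Z scale.
; Tick polls game state to play or reverse a scale timeline, and uses a resettable DoOnce to sound when the cube reaches a set height.
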(event Custom|ScaleUpEvent
  (bind _scalling (Timeline|ScaleUp Play)
    (:Update
      (Transformation|SetActorScale3D _scalling))))

(event Custom|RunLevelConstructionAnim
  (Class|InterptoMovementComponent|RestartMovement (Variables|Default|GetInterpToMovement) 1.0))

(event Custom|ManageObjectScale
  (Transformation|SetRelativeScale3D (Variables|Default|GetCube) (Math|Vector|MakeVector 1.0 1.0 (Math|Random|RandomFloatinRange 1.0 3.0))))

(event EventTick
  (params (DeltaSeconds :type Float%20%28single-precision%29))
  (bind _gamemodereference (Variables|Default|GetGameModeReference))
  (bind _egamestates (Variables|/Game/Blueprints/Game/GM_Arkanoid.GM_Arkanoid_C|GetEGameStates _gamemodereference))
  (Utilities|FlowControl|Sequence
    (:then_0
      (if (Utilities|Enum|Equal(Enum) _egamestates "NewEnumerator1") :!label _label
        (bind _scalling (Timeline|ScaleUp Reverse)
          (:Update
            (Transformation|SetActorScale3D _scalling)))
        (elif (== (.z (Transformation|GetWorldLocation (Variables|Default|GetCube))) 3e+01)
          (Utilities|FlowControl|DoOnce false :!label _label_2
            (:Completed
              (Audio|PlaySound2D "/Game/Sounds/SFX/SC_BlockSpawn.SC_BlockSpawn" 0.75)))
          (else
            (goto _label_2 Reset)))))
    (:then_1
      (if (Utilities|Enum|Equal(Enum) _egamestates "NewEnumerator0")
        (CallFunction|ScaleUpEvent)
        (goto _label)))))

(event EventBeginPlay
  (bind _asgm_arkanoid (Utilities|Casting|CastToGM_Arkanoid (Game|GetGameMode)))
  (bind _output_get (Variables|Default|SetGameModeReference _asgm_arkanoid))
  (EventDispatchers|BindEventtoStartGame _output_get (delegate Custom|RunLevelConstructionAnim))
  (Utilities|Time|SetTimerbyEvent (delegate Custom|ManageObjectScale) (Math|Random|RandomFloatinRange 0.2 0.5) true))

(fn ConstructionScript
  (Variables|/Script/Engine.InterpToMovementComponent|SetDuration (Variables|Default|GetInterpToMovement) (Math|Random|RandomFloatinRange 0.5 2.0)))