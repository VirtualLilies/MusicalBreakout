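; Game mode for an Arkanoid game that runs the match loop: get-ready countdown, score, lives, game over and automatic restart.
; It drives the gameplay UI and player pawn, and saves the high score to a save slot.
; Clearing 30 blocks awards bonus points, an extra life when low, and a timeline-driven slow-motion pitch effect.
; Blocks respawn by unloading and reloading the GameplayBlocks streaming level.
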(event Custom|RestartGame
  (bind _uireference (Variables|Default|GetUIReference))
  ;[0.549 1 0.3961] Reset lifes and score
  (Variables|Game|SetBonusWaves 1)
  (CallFunction|LoadSavedHiScore)
  (Variables|Game|SetEGameStates "NewEnumerator0")
  (Variables|Game|SetBlocksDestroyed 0)
  (Default|SpawnBall (Variables|Default|GetPlayerReference))
  (CallFunction|GetReadyEvent)
  (Default|CallResetPlayerPosition)
  (Default|CallStartGame)
  (CallFunction|LoadGameplayBlocksLevel)
  (Variables|Player|SetCurrentLifes (Variables|Player|GetMaxLifes))
  (Variables|/Game/Blueprints/UI/UI_Gameplay.UI_Gameplay_C|SetScore _uireference 0)
  (Variables|/Game/Blueprints/UI/UI_Gameplay.UI_Gameplay_C|SetLifesLeft _uireference (Variables|Player|GetMaxLifes)))

(event Custom|LoadSavedHiScore
  ;[0.3437 0.4089 1] High score saving
  (bind _returnvalue (SaveGame|DoesSaveGameExist "ScoreSave"))
  (if _returnvalue
    (bind _returnvalue_2 (SaveGame|LoadGamefromSlot "ScoreSave"))
    (bind _asscore_save (Utilities|Casting|CastToScoreSave _returnvalue_2))
    (bind _output_get (Variables|Default|SetScoreSaveReference _asscore_save))
    (Variables|/Game/Blueprints/UI/UI_Gameplay.UI_Gameplay_C|SetHiScore (Variables|Default|GetUIReference) (Utilities|Struct|BreakST_ScoreSave (Variables|/Game/Blueprints/Game/ScoreSave.ScoreSave_C|GetScoreSave _output_get)))
    (else
      (bind _returnvalue_3 (SaveGame|CreateSaveGameObject "/Game/Blueprints/Game/ScoreSave.ScoreSave_C"))
      (Variables|Default|SetScoreSaveReference _returnvalue_3))))

(event Custom|UpdateScore
  (params (Score :type Integer))
  ;[0.549 1 0.3961] Score updating
  (Default|UpdateScoreAnim (Variables|Default|GetUIReference))
  (if (<= (+ Score (Variables|Game|GetCurrentScore)) 0)
    (Variables|Game|SetCurrentScore 0)
    (else
      (Variables|Game|SetCurrentScore (+ Score (Variables|Game|GetCurrentScore)))))
  (Variables|/Game/Blueprints/UI/UI_Gameplay.UI_Gameplay_C|SetScore (Variables|Default|GetUIReference) (Variables|Game|GetCurrentScore)))

(event Custom|GetReadyEvent
  (bind _returnvalue (Game|GetPlayerController 0))
  (bind _playerreference (Variables|Default|GetPlayerReference))
  ;[0.549 1 0.3961] Initial warm up delay
  (Default|GetReadyAnim (Variables|Default|GetUIReference))
  (Input|DisableInput _playerreference _returnvalue)
  (Utilities|FlowControl|Delay 3.0)
  (Input|EnableInput _playerreference _returnvalue)
  (Default|LaunchBall _playerreference)
  (Variables|Game|SetbGameStarted true))

(event Custom|ReloadGameplayBlocks
  (bind _returnvalue (Utilities|Name|MakeLiteralName "GameplayBlocks"))
  ;[0.549 1 0.3961] Reload the blocks when all are taken down
  (Variables|Game|SetBlocksDestroyed 0)
  (Game|UnloadStreamLevel(byName) _returnvalue)
  (if (<= (Variables|Player|GetCurrentLifes) 2)
    (Default|UpdateLifeAnim (Variables|Default|GetUIReference))
    (bind _output_get (Variables|Player|SetCurrentLifes (+ (Variables|Player|GetCurrentLifes) 1)))
    (Variables|/Game/Blueprints/UI/UI_Gameplay.UI_Gameplay_C|SetLifesLeft (Variables|Default|GetUIReference) _output_get))
  (Utilities|FlowControl|Delay 0.5)
  (Game|LoadStreamLevel(byName) _returnvalue true))

(event Custom|OnBonusNotify
  ;[0.549 1 0.3961] Bonus slow motion effect
  (Utilities|FlowControl|Sequence
    (:then_0
      (Utilities|FlowControl|Delay 0.2)
      (bind _customtimedilation (Timeline|SlowTime Play)
        (:Update
          (Class|GameplayStatics|SetGlobalPitchModulation _customtimedilation 0.0)
          (Utilities|Time|SetGlobalTimeDilation _customtimedilation))))
    (:then_1
      (Utilities|FlowControl|Delay 2.5)
      (Timeline|SlowTime Reverse))))

(event Custom|LoadGameplayBlocksLevel
  ;[0.549 1 0.3961] Reload gameplay blocks
  (Game|LoadStreamLevel(byName) (Utilities|Name|MakeLiteralName "GameplayBlocks") true))

(event Custom|DecrimentScore
  ;[0.549 1 0.3961] Decriment score when ball lost, decriment lifes left
  (CallFunction|UpdateScore -250)
  (if (== (Variables|Player|GetCurrentLifes) 1)
    (CallFunction|GameOver)
    (Variables|/Game/Blueprints/UI/UI_Gameplay.UI_Gameplay_C|SetLifesLeft (Variables|Default|GetUIReference) 0)
    (else
      (Default|UpdateLifeAnim (Variables|Default|GetUIReference))
      (bind _output_get (Variables|Player|SetCurrentLifes (- (Variables|Player|GetCurrentLifes) 1)))
      (Variables|/Game/Blueprints/UI/UI_Gameplay.UI_Gameplay_C|SetLifesLeft (Variables|Default|GetUIReference) _output_get))))

(event Custom|GameOver
  (bind _uireference (Variables|Default|GetUIReference))
  ;[0.549 1 0.3961] Run game over state
  (Variables|Game|SetEGameStates "NewEnumerator1")
  (CallFunction|SaveHiScore)
  (Input|DisableInput (Variables|Default|GetPlayerReference) (Game|GetPlayerController 0))
  (Default|RunGameOverAnim _uireference)
  (Default|RunHighScoreAnim _uireference)
  (Audio|PlaySound2D "/Game/Sounds/SFX/S_8Bit_GameOver.S_8Bit_GameOver")
  (Utilities|FlowControl|Delay 3.0)
  (Game|UnloadStreamLevel(byName) (Utilities|Name|MakeLiteralName "GameplayBlocks"))
  (Variables|Game|SetbGameStarted false)
  (CallFunction|RestartGame)
  (Variables|Game|SetCurrentScore 0))

(event Custom|SaveHiScore
  (bind _scoresavereference (Variables|Default|GetScoreSaveReference))
  (bind _currentscore (Variables|Game|GetCurrentScore))
  ;[0.3437 0.4089 1] High score saving
  (if (>= _currentscore (Utilities|Struct|BreakST_ScoreSave (Variables|/Game/Blueprints/Game/ScoreSave.ScoreSave_C|GetScoreSave (stale Custom|LoadSavedHiScore _output_get))))
    (Variables|/Game/Blueprints/Game/ScoreSave.ScoreSave_C|SetScoreSave _scoresavereference (Utilities|Struct|MakeST_ScoreSave _currentscore))
    (SaveGame|SaveGametoSlot _scoresavereference "ScoreSave")))

(event EventBeginPlay
  ;[1 0.3961 0.3961] Load score save and add UI on begin play
  (bind _returnvalue (UserInterface|CreateWidget "/Game/Blueprints/UI/UI_Gameplay.UI_Gameplay_C"))
  (bind _output_get (Variables|Default|SetUIReference _returnvalue))
  (UserInterface|Viewport|AddtoViewport _output_get 0)
  ;[1 0.3961 0.3961] Disable mouse cursor, focus on game input
  (bind _asbp_pc (Utilities|Casting|CastToBP_PC (Game|GetPlayerController 0)))
  (Input|SetInputModeGameOnly _asbp_pc)
  (Variables|/Script/Engine.PlayerController|SetbShowMouseCursor _asbp_pc false)
  ;[1 0.3961 0.3961] Save player reference
  (bind _asbp_player (Utilities|Casting|CastToBP_Player (Game|Player|GetPlayerPawn 0)))
  (Variables|Default|SetPlayerReference _asbp_player)
  ;[1 0.3961 0.3961] Run the game
  (CallFunction|RestartGame))

(event EventBlockWasDestroyed
  (bind _uireference (Variables|Default|GetUIReference))
  ;[0.549 1 0.3961] Blocks destroy count, used for respawning blocks when all are destroyed
  (Variables|Game|SetBlocksDestroyed (+ (Variables|Game|GetBlocksDestroyed) 1))
  (if (>= (Variables|Game|GetBlocksDestroyed) 30)
    (if (Utilities|Enum|NotEqual(Enum) (Variables|Game|GetEGameStates) "NewEnumerator1")
      (CallFunction|OnBonusNotify)
      (Default|PlayBonusNotification _uireference)
      (Default|BonusUpdateAnim _uireference)
      (bind _output_get (Variables|Game|SetBonusWaves (+ (Variables|Game|GetBonusWaves) 1)))
      (CallFunction|BonusWave _output_get)
      (CallFunction|UpdateScore 5000)
      (CallFunction|ReloadGameplayBlocks))))

(fn ConstructionScript)