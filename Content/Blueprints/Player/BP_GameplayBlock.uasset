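; Destructible Arkanoid block that scales in on BeginPlay and has a three-mesh body tinted through dynamic materials.
; Tick enables collision with a spawn sound once root Z reaches zero, or reverses the scale timeline in one game state.
; Ball hits trigger audio and camera shake.
; The first end overlap adds score, breaks the meshes into spinning physics pieces, notifies GM_Arkanoid and sets a short lifespan.
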(event OnComponentEndOverlap(CollisionVolume)
  (params (OverlappedComponent :type Primitive%20Component%20Object%20Reference) (OtherActor :type Actor%20Object%20Reference) (OtherComp :type Primitive%20Component%20Object%20Reference) (OtherBodyIndex :type Integer))
  (bind _gamemodereference (Variables|Default|GetGameModeReference))
  ;[1 0.2235 0.2235] Add score per block to total score
  (bind _asgm_arkanoid (Utilities|Casting|CastToGM_Arkanoid (Game|GetGameMode)))
  (Utilities|FlowControl|DoOnce false ; Make sure to not colide twice with the block
    (:Completed
      (Default|UpdateScore _asgm_arkanoid (Variables|Scoring|GetScore))
      ;[1 0.2235 0.2235] Handle destroy mechanic on gameplay block hit
      (CallFunction|SimulatePhysicsonBlocks)
      (Utilities|IsValid _gamemodereference
        (:Is%20Valid
          (Default|BlockWasDestroyed _gamemodereference)
          (Actor|SetLifeSpan 2.0))))))

(event Custom|ScaleUp
  ;[1 1 1] Scale up
  (bind _scalling (Timeline|InitialScale Play)
    (:Update
      (Transformation|SetActorScale3D _scalling))))

(event EventBeginPlay
  ;[1 0.2235 0.2235] Store gameplay block location
  (Variables|BlockDefaults|SetGameplayBlockInitialLocation (Transformation|GetActorLocation))
  ;[1 0.2235 0.2235] Save game mode reference
  (bind _asgm_arkanoid (Utilities|Casting|CastToGM_Arkanoid (Game|GetGameMode)))
  (Variables|Default|SetGameModeReference _asgm_arkanoid)
  (CallFunction|ScaleUp))

(event Collision|EventHit
  (params (MyComp :type Primitive%20Component%20Object%20Reference) (Other :type Actor%20Object%20Reference) (OtherComp :type Primitive%20Component%20Object%20Reference) (bSelfMoved :type Boolean) (HitLocation :type Vector) (HitNormal :type Vector :default "0, 0, 0") (NormalImpulse :type Vector :default "0, 0, 0") (Hit :type Hit%20Result%20Structure%20%28by%20ref%29))
  ;[1 0.2235 0.2235] Play SFX and camera shake on block hit
  (Utilities|Casting|CastToBP_Ball Other)
  (Audio|Components|Audio|Play (Variables|Default|GetAudio) 0.0)
  (Camera|PlayWorldCameraShake "/Game/Blueprints/Player/BP_BlockHit_CM.BP_BlockHit_CM_C" HitLocation 5e+03 0.0))

(event EventTick
  (params (DeltaSeconds :type Float%20%28single-precision%29))
  ;[1 0 0] Event Tick
  ;[1 0.2235 0.2235] Play spawn sound fx
  (if (Utilities|Enum|Equal(Enum) (Variables|/Game/Blueprints/Game/GM_Arkanoid.GM_Arkanoid_C|GetEGameStates (Variables|Default|GetGameModeReference)) "NewEnumerator1")
    ;[1 1 1] Scale up
    (bind _scalling (Timeline|InitialScale Reverse)
      (:Update
        (Transformation|SetActorScale3D _scalling)))
    (elif (== (.z (Variables|/Script/Engine.SceneComponent|GetRelativeLocation (Variables|Default|GetDefaultSceneRoot))) 0.0)
      (Utilities|FlowControl|DoOnce false
        (:Completed
          (Audio|PlaySound2D "/Game/Sounds/SFX/SC_BlockSpawn.SC_BlockSpawn")
          (Collision|SetCollisionEnabled (Variables|Default|GetCollisionVolume) "QueryAndPhysics"))))))

(fn ConstructionScript
  (Collision|SetCollisionEnabled (Variables|Default|GetCollisionVolume) "NoCollision")
  (bind _returnvalue (Rendering|Material|CreateDynamicMaterialInstance (Variables|Default|GetBlock_01) 0 "/Game/Materials/M_BaseColor.M_BaseColor" :!class /Script/Engine.PrimitiveComponent))
  (bind _output_get (LocalVariables|SetMID_01 _returnvalue))
  (Rendering|Material|SetVectorParameterValue _output_get "Color" (Variables|BlockDefaults|GetColor) :!class /Script/Engine.MaterialInstanceDynamic)
  (bind _returnvalue_2 (Rendering|Material|CreateDynamicMaterialInstance (Variables|Default|GetBlock_02) 0 "/Game/Materials/M_BaseColor.M_BaseColor" :!class /Script/Engine.PrimitiveComponent))
  (bind _output_get_2 (LocalVariables|SetMID_02 _returnvalue_2))
  (Rendering|Material|SetVectorParameterValue _output_get_2 "Color" (Variables|BlockDefaults|GetColor) :!class /Script/Engine.MaterialInstanceDynamic)
  (bind _returnvalue_3 (Rendering|Material|CreateDynamicMaterialInstance (Variables|Default|GetBlock_03) 0 "/Game/Materials/M_BaseColor.M_BaseColor" :!class /Script/Engine.PrimitiveComponent))
  (bind _output_get_3 (LocalVariables|SetMID_03 _returnvalue_3))
  (Rendering|Material|SetVectorParameterValue _output_get_3 "Color" (Variables|BlockDefaults|GetColor) :!class /Script/Engine.MaterialInstanceDynamic)
  (Variables|/Script/Engine.InterpToMovementComponent|SetDuration (Variables|Default|GetInterpToMovement) (Math|Random|RandomFloatinRange 2.0 3.0)))

(fn SimulatePhysicsonBlocks
  (bind _returnvalue (Math|Random|RandomFloatinRange -2.0 2.0))
  (bind _returnvalue_2 (Math|Random|RandomFloatinRange -2.0 2.0))
  (bind _returnvalue_3 (Math|Random|RandomFloatinRange -2.0 2.0))
  (bind _block_02 (Variables|Default|GetBlock_02))
  (bind _block_03 (Variables|Default|GetBlock_03))
  (bind _block_01 (Variables|Default|GetBlock_01))
  (Physics|SetSimulatePhysics _block_01 true)
  (Class|PrimitiveComponent|AddAngularImpulse _block_01 (Math|Vector|MakeVector _returnvalue_2 _returnvalue_2 _returnvalue_2) "None" true)
  (Physics|SetSimulatePhysics _block_02 true)
  (Class|PrimitiveComponent|AddAngularImpulse _block_02 (Math|Vector|MakeVector _returnvalue_3 _returnvalue_3 _returnvalue_3) "None" true)
  (Physics|SetSimulatePhysics _block_03 true)
  (Class|PrimitiveComponent|AddAngularImpulse _block_03 (Math|Vector|MakeVector _returnvalue _returnvalue _returnvalue) "None" true))