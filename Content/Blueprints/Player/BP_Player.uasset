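; Player paddle pawn for an Arkanoid-style game that moves horizontally, spawns and launches the ball, and handles pause and level restart.
; Axis input pushes the BlockCenter block with impulses while the game mode state allows, and a game mode dispatcher resets its position.
; Balls launch at a random diagonal with sound and camera shake.
; Unpausing ramps time dilation via timeline, and construction tints the paddle per level name.
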(event Custom|SpawnBall
  ;[0.5961 1 0.349] Spawn gameplay ball event
  (if (Utilities|Enum|Equal(Enum) (Variables|/Game/Blueprints/Game/GM_Arkanoid.GM_Arkanoid_C|GetEGameStates (Variables|Default|GetGameModeReference)) "NewEnumerator0")
    (bind _returnvalue (Game|SpawnActorfromClass "/Game/Blueprints/Player/BP_Ball.BP_Ball_C" (Math|Transform|MakeTransform (+ (Transformation|GetWorldLocation (Variables|Default|GetBallSpawnPoint)) "0.000000,-150.000000, 0") "0, 0, 0" "1,1,1") "AlwaysSpawn" 0 0))
    (Variables|Default|SetBallReference _returnvalue)
    (if (Variables|/Game/Blueprints/Game/GM_Arkanoid.GM_Arkanoid_C|GetbGameStarted (Variables|Default|GetGameModeReference))
      (CallFunction|LaunchBall))))

(event Custom|ResetPlayerPosition
  (bind _playerstartlocation (Variables|Player|GetPlayerStartLocation))
  ;[0.5961 1 0.349] Reset player position event
  (Transformation|SetActorLocation _playerstartlocation false false)
  (Transformation|SetWorldLocation (Variables|Default|GetBlock_Center) _playerstartlocation false false))

(event Custom|UnpauseGame
  ;[0.5961 1 0.349] Game Pause
  (bind _speedupgameplay (Timeline|PauseExitSpeedUp PlayFromStart)
    (:Update
      (Utilities|Time|SetGlobalTimeDilation _speedupgameplay)
      (Game|SetGamePaused false))))

(event Custom|LaunchBall
  (bind _ballreference (Variables|Default|GetBallReference))
  (bind _ballspawnpoint (Variables|Default|GetBallSpawnPoint))
  ;[0.5961 1 0.349] Launch the ball
  (if (and (Utilities|IsValid _ballreference) (not (Variables|/Game/Blueprints/Player/BP_Ball.BP_Ball_C|GetbIsBallActive _ballreference)))
    (Utilities|FlowControl|Delay 0.33)
    (Transformation|SetRelativeRotation _ballspawnpoint (select (Math|Random|RandomBool) "0.000000,-45.000000,0.000000" "0,45.000000,0") false false)
    (Audio|PlaySound2D "/Game/Sounds/SFX/S_8Bit_BallLaunch.S_8Bit_BallLaunch")
    (Default|LaunchBall _ballreference (Math|Rotator|GetRotationXVector (Transformation|GetWorldRotation _ballspawnpoint)))
    (Camera|PlayWorldCameraShake "/Game/Blueprints/Player/BP_BallLaunch_CM.BP_BallLaunch_CM_C" "0, 0, 0" 5e+03 0.0)))

(event EventBeginPlay
  ;[1 0.27 0.27] Begin Play
  ;[0.5373 0.5333 1] Save game mode reference
  (bind _asgm_arkanoid (Utilities|Casting|CastToGM_Arkanoid (Game|GetGameMode)))
  (Variables|Default|SetGameModeReference _asgm_arkanoid)
  ;[0.5373 0.5333 1] Save player starting position
  (Variables|Player|SetPlayerStartLocation (Transformation|GetActorLocation))
  ;[0.5373 0.5333 1] Listen to the dispatchers
  (EventDispatchers|BindEventtoResetPlayerPosition (Variables|Default|GetGameModeReference) (delegate Custom|ResetPlayerPosition)))

(event Input|ActionEvents|InputActionRestart
  (params (Key :type Key%20Structure :default "AnyKey"))
  ;[0.5961 1 0.349] Restart the game through button input
  (:Pressed
    (bind _returnvalue (Game|GetCurrentLevelName true))
    (Game|OpenLevel(byName) (Utilities|String|StringToName _returnvalue))))

(event Input|ActionEvents|InputActionPause
  (params (Key :type Key%20Structure :default "AnyKey"))
  ;[0.5961 1 0.349] Game Pause
  (:Pressed
    (CallFunction|PauseGame)))

(event Input|AxisEvents|InputAxisMoveHorizontal
  (params (AxisValue :type Float%20%28single-precision%29))
  ;[0.5961 1 0.349] Player paddle movement
  (if (Utilities|Enum|Equal(Enum) (Variables|/Game/Blueprints/Game/GM_Arkanoid.GM_Arkanoid_C|GetEGameStates (Variables|Default|GetGameModeReference)) "NewEnumerator0")
    (Physics|AddImpulse (Variables|Default|GetBlock_Center) (Math|Vector|MakeVector (* AxisValue (Variables|Player|GetSpeed)) 0.0 0.0) "None" false)))

(fn ConstructionScript
  (bind _block_center (Variables|Default|GetBlock_Center))
  (bind _returnvalue (Game|GetCurrentLevelName true))
  (switch string _returnvalue
    (:GameplayGangam
      (bind _returnvalue_2 (Rendering|Material|CreateDynamicMaterialInstance _block_center 0 "/Game/Materials/M_BaseColor.M_BaseColor" :!class /Script/Engine.PrimitiveComponent))
      (bind _output_get (LocalVariables|SetMID_BlockCenter _returnvalue_2))
      (Rendering|Material|SetVectorParameterValue _output_get "Color" "(R=0.647059,G=0.000000,B=0.000000,A=1.000000)" :!class /Script/Engine.MaterialInstanceDynamic))
    (:GamePlayShapeOfYou
      (bind _returnvalue_3 (Rendering|Material|CreateDynamicMaterialInstance _block_center 0 "/Game/Materials/M_BaseColor.M_BaseColor" :!class /Script/Engine.PrimitiveComponent))
      (bind _output_get_2 (LocalVariables|SetMID_BlockCenter _returnvalue_3))
      (Rendering|Material|SetVectorParameterValue _output_get_2 "Color" "(R=1.000000,G=1.000000,B=1.000000,A=1.000000)" :!class /Script/Engine.MaterialInstanceDynamic))
    (:GameplayPowerRangers
      (bind _returnvalue_4 (Rendering|Material|CreateDynamicMaterialInstance _block_center 0 "/Game/Materials/M_BaseColor.M_BaseColor" :!class /Script/Engine.PrimitiveComponent))
      (bind _output_get_3 (LocalVariables|SetMID_BlockCenter _returnvalue_4))
      (Rendering|Material|SetVectorParameterValue _output_get_3 "Color" "(R=0.104814,G=0.670000,B=0.000000,A=1.000000)" :!class /Script/Engine.MaterialInstanceDynamic))))

(fn PauseGame
  (bind _returnvalue (Game|GetPlayerController 0))
  (Game|SetGamePaused true)
  (Utilities|IsValid (Variables|Default|GetPauseMenuReference)
    (:Is%20Valid
      _)
    (:Is%20Not%20Valid
      (bind _returnvalue_2 (UserInterface|CreateWidget "/Game/Blueprints/UI/UI_PauseMenu.UI_PauseMenu_C" _returnvalue))
      (bind _output_get (Variables|Default|SetPauseMenuReference _returnvalue_2))))
  (UserInterface|Viewport|AddtoViewport _output_get 1)
  (Input|SetInputModeUIOnly _returnvalue _output_get "DoNotLock")
  (Variables|/Script/Engine.PlayerController|SetbShowMouseCursor _returnvalue true)
  (Default|RunPauseMenuAnim (Variables|Default|GetPauseMenuReference)))

(fn RemovePauseUI
  (bind _returnvalue (Game|GetPlayerController 0))
  (Widget|RemovefromParent (Variables|Default|GetPauseMenuReference))
  (Input|SetInputModeGameOnly _returnvalue)
  (Variables|/Script/Engine.PlayerController|SetbShowMouseCursor _returnvalue false))